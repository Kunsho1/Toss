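; Press trap for TossGame that slams a press down and kills living BPEnemyAI it hits, then recharges.
; ActivateTrap runs a working timeline lerping the press from its start transform to a lowered one, then a recharging timeline also drives it between them.
; Hits only kill while the trap is active and deadly, calling the enemy's status component death.
; When recharging finishes, it marks itself and its linked button ready again.
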(event `self.ReceiveBeginPlay`
  (bind (_returnvalue_location _returnvalue_rotation _returnvalue_scale) (`KismetMathLibrary.BreakTransform` (`SceneComponent.GetRelativeTransform` (`self.Press`))))
  (set `self.BasePosition` (`KismetMathLibrary.MakeTransform` _returnvalue_location _returnvalue_rotation _returnvalue_scale))
  (set `self.FinalPosition` (`KismetMathLibrary.MakeTransform` (- _returnvalue_location (0.0 0.0 370.0)) _returnvalue_rotation _returnvalue_scale))
  (set `self.IsActive` false)
  (set `self.IsReady` true))

(event `Activate Trap`
  (set `self.IsActive` true)
  (set `self.IsReady` false)
  (bind (_direction _trapmovement) (`Timeline|TrapWorking` :!via `PlayFromStart`)
    (:`Update`
      (`SceneComponent.K2_SetRelativeTransform` (`self.Press`) (`KismetMathLibrary.TLerp` (`self.BasePosition`) (`self.FinalPosition`) _trapmovement) false false))
    (:`Finished`
      (set `self.IsActive` false)
      (bind (_direction_2 _trapmovement_2) (`Timeline|TrapRecharging` :!via `PlayFromStart`)
        (:`Update`
          (`SceneComponent.K2_SetRelativeTransform` (`self.Press`) (`KismetMathLibrary.TLerp` (`self.BasePosition`) (`self.FinalPosition`) _trapmovement_2) false false))
        (:`Finished`
          (set `self.IsReady` true)
          (set `/Game/TossGame/Traps/ButtonBP.IsReady` true (`self.MyButton`)))))))

(event `self.Press.OnComponentHit`
  (params (HitComponent :type "PrimitiveComponent Object Reference") (OtherActor :type "Actor Object Reference") (OtherComp :type "PrimitiveComponent Object Reference") (NormalImpulse :type "Vector Structure") (Hit :type "HitResult Structure (by ref)"))
  (if (and (`self.IsActive`) (`self.IsDeadly`))
    (bind _asbpenemy_ai (cast `/Game/TossGame/Enemies/BPEnemyAI` OtherActor))
    (if (`/Game/TossGame/Enemies/BPEnemyAI.IsAlive` _asbpenemy_ai)
      (`/Game/TossGame/Enemies/StatusAC.OnDeath` (`/Game/TossGame/Enemies/BPEnemyAI.StatusAC` _asbpenemy_ai))
      (`KismetSystemLibrary.PrintString` "Squish"))))

(fn `UserConstructionScript`)