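; Pressure button that activates its linked traps when a NormalCube hits it.
; BeginPlay registers the button with each trap and caches pressed and rest transforms.
; A hit fires every trap, clears readiness and runs a timeline macro that pushes the button down and back up.
; Tick feeds a material "State" parameter showing ready, pressed or waiting; nothing here restores readiness after a press.
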(event `self.ReceiveBeginPlay`
  (bind (_returnvalue_location _returnvalue_rotation _returnvalue_scale) (`KismetMathLibrary.BreakTransform` (`SceneComponent.GetRelativeTransform` (`self.Button`))))
  (set `self.InPosition` (`KismetMathLibrary.MakeTransform` _returnvalue_location _returnvalue_rotation _returnvalue_scale))
  (set `self.OutPosition` (`KismetMathLibrary.MakeTransform` (- _returnvalue_location (0.0 0.0 8.0)) _returnvalue_rotation _returnvalue_scale))
  (for _array_element (`self.Traps`)
    (set `/Game/TossGame/Traps/PressTrapBP.MyButton` self _array_element))
  (set `self.IsReady` true)
  (set `self.ButtonState` 0.0))

(event `self.Button.OnComponentHit`
  (params (HitComponent :type "PrimitiveComponent Object Reference") (OtherActor :type "Actor Object Reference") (OtherComp :type "PrimitiveComponent Object Reference") (NormalImpulse :type "Vector Structure") (Hit :type "HitResult Structure (by ref)"))
  (if (`self.IsReady`)
    (cast `/Game/TossGame/Throwables/NormalCube` OtherActor)
    (`KismetSystemLibrary.PrintString` "Hello")
    (for _array_element (`self.Traps`)
      (`/Game/TossGame/Traps/PressTrapBP.Activate Trap` _array_element))
    (set `self.IsReady` false)
    (set `self.ButtonState` 1.0)
    (bind (_direction _button_in) (`Timeline|Button In` :!via `PlayFromStart`)
      (:`Update`
        (`SceneComponent.K2_SetRelativeTransform` (`self.Button`) (`KismetMathLibrary.TLerp` (`self.InPosition`) (`self.OutPosition`) _button_in) false false))
      (:`Finished`
        (bind (_direction_2 _button_in_2) (`Timeline|Button Out` :!via `ReverseFromEnd`)
          (:`Update`
            (`SceneComponent.K2_SetRelativeTransform` (`self.Button`) (`KismetMathLibrary.TLerp` (`self.InPosition`) (`self.OutPosition`) _button_in_2) false false))
          (:`Finished`
            (set `self.ButtonState` 0.5)))))))

(event `self.ReceiveTick`
  (params (DeltaSeconds :type "Float (single-precision)"))
  (`|ExecutionSequence`
    (:`then_0`
      (if (`self.IsReady`)
        (set `self.ButtonState` 0.0)))
    (:`then_1`
      (`MeshComponent.SetScalarParameterValueOnMaterials` (`self.Button`) "State" (`self.ButtonState`)))))

(fn `UserConstructionScript`)